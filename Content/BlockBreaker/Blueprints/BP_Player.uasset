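; First-person player for BlockBreaker that handles movement, mouse look, weapon swapping and shooting.
; It spawns a rifle on GunLocation at BeginPlay, and swap inputs destroy the held gun and spawn a fresh rifle or shotgun.
; Shooting passes camera-forward trace endpoints to the gun's Shoot, spends ammo and gates fire with a FireRate delay.
; An empty gun refills after ReloadTime without a separate reload input.
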(event `InputAxis|SwapRifle`
  (params (AxisValue :type "Float (single-precision)"))
  ;[1 1 1] Swap Gun
  (if (== AxisValue 1.0)
    (`self.K2_DestroyActor` (`self.EquippedGun`))
    (bind _returnvalue (`|SpawnActorFromClass` "/Game/BlockBreaker/Blueprints/BP_Rifle.BP_Rifle_C" (`KismetMathLibrary.MakeTransform` (0.0 0.0 0.0)) "Undefined" "OverrideRootScale" null null))
    (bind _output_get (set `self.EquippedGun` _returnvalue))
    (`self.K2_AttachToComponent` _output_get (`self.GunLocation`) "None" "KeepRelative" "KeepRelative" "KeepRelative" true)))

(event `InputAxis|MoveForward`
  (params (AxisValue :type "Float (single-precision)"))
  ;[1 1 1] Movement WASD
  (`self.AddMovementInput` (`self.GetActorForwardVector`) AxisValue))

(event `self.ReceiveBeginPlay`
  ;[1 1 1] Spawn and Attach Weapon
  (bind _returnvalue (`|SpawnActorFromClass` "/Game/BlockBreaker/Blueprints/BP_Rifle.BP_Rifle_C" (`KismetMathLibrary.MakeTransform` (0.0 0.0 0.0)) "Undefined" "OverrideRootScale" null null))
  (bind _output_get (set `self.EquippedGun` _returnvalue))
  (`self.K2_AttachToComponent` _output_get (`self.GunLocation`) "None" "SnapToTarget" "SnapToTarget" "KeepRelative" true))

(event `InputAxis|MoveRight`
  (params (AxisValue :type "Float (single-precision)"))
  ;[1 1 1] Movement WASD
  (`self.AddMovementInput` (`self.GetActorRightVector`) AxisValue))

(event `InputAxis|SwapShotgun`
  (params (AxisValue :type "Float (single-precision)"))
  ;[1 1 1] Swap Gun
  (if (== AxisValue 1.0)
    (`self.K2_DestroyActor` (`self.EquippedGun`))
    (bind _returnvalue (`|SpawnActorFromClass` "/Game/BlockBreaker/Blueprints/BP_Shotgun.BP_Shotgun_C" (`KismetMathLibrary.MakeTransform` (0.0 0.0 0.0)) "Undefined" "OverrideRootScale" null null))
    (bind _output_get (set `self.EquippedGun` _returnvalue))
    (`self.K2_AttachToComponent` _output_get (`self.GunLocation`) "None" "KeepRelative" "KeepRelative" "KeepRelative" true)))

(event `InputAxis|Shoot`
  (params (AxisValue :type "Float (single-precision)"))
  (bind _fpscamera (`self.FpsCamera`))
  (bind _returnvalue (`SceneComponent.K2_GetComponentLocation` _fpscamera))
  (bind _ammo (`/Game/BlockBreaker/Blueprints/BP_BaseGun.Ammo` (`self.EquippedGun`)))
  ;[1 1 1] Shoot
  (if (and (== AxisValue 1.0) (`self.CanShoot`) (>= _ammo 1.0))
    (`/Game/BlockBreaker/Blueprints/BP_BaseGun.Shoot` (`self.EquippedGun`) _returnvalue (+ _returnvalue (* (`SceneComponent.GetForwardVector` _fpscamera) (`/Game/BlockBreaker/Blueprints/BP_BaseGun.MaxBulletDistance` (`self.EquippedGun`)))))
    (set `/Game/BlockBreaker/Blueprints/BP_BaseGun.Ammo` (- (`/Game/BlockBreaker/Blueprints/BP_BaseGun.Ammo` (`self.EquippedGun`)) 1.0) (`self.EquippedGun`))
    (set `self.CanShoot` false)
    ;[1 1 1] Swap Gun
    (`KismetSystemLibrary.Delay` (`/Game/BlockBreaker/Blueprints/BP_BaseGun.FireRate` (`self.EquippedGun`)))
    (set `self.CanShoot` true)
    (else
      ;[1 1 1] Reload
      (if (<= _ammo 0.0)
        (set `self.Reloading` true)
        (`KismetSystemLibrary.Delay` (`/Game/BlockBreaker/Blueprints/BP_BaseGun.Reload time` (`self.EquippedGun`)))
        (set `self.Reloading` false)
        (set `/Game/BlockBreaker/Blueprints/BP_BaseGun.Ammo` (`/Game/BlockBreaker/Blueprints/BP_BaseGun.MaxAmmo` (`self.EquippedGun`)) (`self.EquippedGun`))))))

(event `InputAxis|LookHorizontal`
  (params (AxisValue :type "Float (single-precision)"))
  ;[1 1 1] Look Mapping (mouse)
  (`self.AddControllerYawInput` AxisValue))

(event `InputAxis|LookVertical`
  (params (AxisValue :type "Float (single-precision)"))
  ;[1 1 1] Look Mapping (mouse)
  (`self.AddControllerPitchInput` (* AxisValue -1.0)))

(fn `UserConstructionScript`)